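; Enemy Blueprint that tracks health and is destroyed when that health runs out.
; TakeDamage prints a debug string, subtracts the given amount from Health, then destroys the actor if CheckIfDead finds Health at or below zero.
; BeginPlay only prints a taunt, while overlap, Tick and the construction script are empty.
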(event Custom|TakeDamage
  (params (ByAmount :type Float%20%28double-precision%29))
  (Development|PrintString "damn")
  (Variables|Default|SetHealth (- (Variables|Default|GetHealth) ByAmount))
  (if (CallFunction|CheckifDead (Variables|Default|GetHealth))
    (Actor|DestroyActor)))

(event EventBeginPlay
  (Development|PrintString "Die Now! Bitch"))

(event Collision|EventActorBeginOverlap
  (params (OtherActor :type Actor%20Object%20Reference)))

(event EventTick
  (params (DeltaSeconds :type Float%20%28single-precision%29)))

(fn ConstructionScript)

(fn CheckifDead
  (params (Health :type Float%20%28double-precision%29))
  (return (<= Health 0.0)))