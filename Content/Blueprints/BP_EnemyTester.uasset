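; BP_EnemyTester is a test actor that repeatedly damages every BP_Enemy in the level.
; From BeginPlay, it gathers all BP_Enemy actors, prints their count and calls TakeDamage on each with a small random amount.
; It prints a confirmation, waits on a Delay, then calls its GiveDamage event again, forming an endless timed loop that re-queries the enemies each pass.
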(event Custom|GiveDamage
  (bind _outactors (Actor|GetAllActorsOfClass "/Game/Blueprints/BP_Enemy.BP_Enemy_C")) ; Find all of the BP_Enemies
  (Development|PrintString (Utilities|String|Append "therw" (Utilities|String|ToString(Integer) (Utilities|Array|Length _outactors)) "are 1"))
  (for _array_element _outactors
    (Default|TakeDamage _array_element (Math|Random|RandomFloatinRange 0.1 2.0)))
  (Development|PrintString "we've given damage to all the enmies")
  (Utilities|FlowControl|Delay 2.0)
  (CallFunction|GiveDamage))

(event EventBeginPlay
  (bind _outactors (Actor|GetAllActorsOfClass "/Game/Blueprints/BP_Enemy.BP_Enemy_C")) ; Find all of the BP_Enemies
  (Development|PrintString (Utilities|String|Append "therw" (Utilities|String|ToString(Integer) (Utilities|Array|Length _outactors)) "are 1"))
  (for _array_element _outactors
    (Default|TakeDamage _array_element (Math|Random|RandomFloatinRange 0.1 2.0)))
  (Development|PrintString "we've given damage to all the enmies")
  (Utilities|FlowControl|Delay 2.0)
  (CallFunction|GiveDamage))

(event Collision|EventActorBeginOverlap
  (params (OtherActor :type Actor%20Object%20Reference)))

(event EventTick
  (params (DeltaSeconds :type Float%20%28single-precision%29)))

(fn ConstructionScript)