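; BP_Item2 is an item that can be picked up, carried and dropped, with a Cube component as its physical body.
; PickUp disables the Cube's collision and snaps it to the `item_socket_right` socket on the given parent.
; Drop detaches the Cube, restores collision, enables physics and applies a fixed forward-and-up force along world axes, ignoring mass.
; PrimaryAction is a stub that only prints a debug string.
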(event Custom|PickUp
  (params (Parent :type Scene%20Component%20Object%20Reference))
  ;[1 1 1] Comment
  (Development|PrintString "Pickup")
  (Collision|SetCollisionEnabled (Variables|Default|GetCube) "NoCollision")
  (Transformation|AttachComponentToComponent Parent "item_socket_right" "SnapToTarget" "SnapToTarget" "KeepRelative" true))

(event Custom|Drop
  (Development|PrintString "Drop")
  (Transformation|DetachFromComponent (Variables|Default|GetCube) "KeepWorld" "KeepWorld" "KeepRelative" true)
  (Collision|SetCollisionEnabled (Variables|Default|GetCube) "QueryAndPhysics")
  (Physics|SetSimulatePhysics (Variables|Default|GetCube) true)
  (Physics|AddForce (Variables|Default|GetCube) "1000.000000,0.000000,500.000000" "None" true))

(event Custom|PrimaryAction
  (Development|PrintString "Action!"))

(fn ConstructionScript)