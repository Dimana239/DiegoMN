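; BP_Item is a carriable item with pickup, drop and an empty PrimaryAction event.
; Pickup disables the Cube's collision so it cannot push the carrier, then snaps it to the item_socket_r socket on the passed CapsuleComponent.
; Drop restores physics-only collision, detaches the Cube in world space, re-enables simulation and tosses it with a fixed world-axis force applied as acceleration.
; Both events print debug messages.
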(event Custom|Pickup
  (params (CapsuleComponent :type Scene%20Component%20Object%20Reference%20%28by%20ref%29))
  (Development|PrintString "Picked Up!")
  (Collision|SetCollisionEnabled (Variables|Default|GetCube) "NoCollision") ; Don't push us off the map
  (Transformation|AttachComponentToComponent CapsuleComponent "item_socket_r" "SnapToTarget" "SnapToTarget" "KeepRelative" true))

(event Custom|Drop
  (Development|PrintString "dropped" true true "(R=0.723214,G=0.015693,B=0.000000,A=1.000000)" 6.0)
  (Collision|SetCollisionEnabled (Variables|Default|GetCube) "PhysicsOnly")
  (Physics|SetSimulatePhysics (Variables|Default|GetCube) false)
  (Transformation|DetachFromComponent (Variables|Default|GetCube) "KeepWorld" "KeepRelative" "KeepRelative" true)
  (Physics|SetSimulatePhysics (Variables|Default|GetCube) true)
  (Physics|AddForce (Variables|Default|GetCube) "500.000000,0.000000,250.000000" "None" true))

(event Custom|PrimaryAction)

(fn ConstructionScript)